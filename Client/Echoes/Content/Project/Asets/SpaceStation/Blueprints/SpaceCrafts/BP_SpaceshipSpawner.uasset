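; Spaceship spawner actor that previews the chosen spacecraft class as a placeholder mesh and spawns it at its own location and rotation.
; The construction script briefly creates a child actor to copy the spacecraft's mesh, then destroys it.
; An optional box trace around the placeholder picks a valid or invalid material to show blocked placement.
; SpawnSpaceship destroys any previously spawned ship before spawning another, without checking for blockage.
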(event `SpawnSpaceship`
  (bind _spawnedspaceship (`self.SpawnedSpaceship`))
  (`/Engine/EditorBlueprintResources/StandardMacros.IsValid` _spawnedspaceship
    (:`Is Valid`
      (`self.K2_DestroyActor` _spawnedspaceship))
    (:`Is Not Valid`
      _))
  (`self.SpawnActor`))

(event `self.ReceiveTick`
  (params (DeltaSeconds :type "Float (single-precision)")))

(fn `CheckIfBlocking`
  (bind _returnvalue (`self.K2_GetActorLocation`))
  (if (`self.AllowChecking`)
    (bind (_outhit _returnvalue_2) (`KismetSystemLibrary.BoxTraceSingle` :`Start` _returnvalue :`End` _returnvalue :`HalfSize` (* (`.BoxExtent` (`KismetSystemLibrary.GetComponentBounds` (`self.PlaceholderShipMesh`))) 2.0) :`Orientation` (`self.K2_GetActorRotation`) :`TraceChannel` "TraceTypeQuery1" :`DrawDebugType` "ForOneFrame"))
    (set `self.SomethingBlocking` _returnvalue_2)))

(fn `SpawnActor`
  (bind _returnvalue (`|SpawnActorFromClass` (`self.SpaceshipActorToSpawn`) (`KismetMathLibrary.MakeTransform` (`self.K2_GetActorLocation`) (`self.K2_GetActorRotation`)) "Undefined" "SelectDefaultAtRuntime" null null))
  (bind _output_get (set `self.SpawnedSpaceship` _returnvalue))
  (cast `/Game/Project/Asets/SpaceStation/Blueprints/SpaceCrafts/Parent/BP_ParentSpacecraft` _output_get))

(fn `UserConstructionScript`
  (bind _placeholdershipmesh (`self.PlaceholderShipMesh`))
  (if (`KismetSystemLibrary.IsValidClass` (`self.SpaceshipActorToSpawn`))
    ;[1 1 1] Spawn Temporal child ship actor
    (bind _returnvalue (`AddComponent|NODE_AddChildActorComponent-0` :`RelativeTransform` (`SceneComponent.GetRelativeTransform` (`self.PlaceholderShipMesh`))))
    (bind _output_get (set `self.PlaceholderActor` _returnvalue))
    (`ChildActorComponent.SetChildActorClass` _output_get (`self.SpaceshipActorToSpawn`))
    (bind _asbp_parent_spacecraft (cast `/Game/Project/Asets/SpaceStation/Blueprints/SpaceCrafts/Parent/BP_ParentSpacecraft` (`ChildActorComponent.ChildActor` (`self.PlaceholderActor`))))
    ;[1 1 1] Set Placeholder ship mesh
    (`StaticMeshComponent.SetStaticMesh` (`self.PlaceholderShipMesh`) (`StaticMeshComponent.StaticMesh` (`/Game/Project/Asets/SpaceStation/Blueprints/SpaceCrafts/Parent/BP_ParentSpacecraft.Plane mesh` _asbp_parent_spacecraft)))
    (`self.CheckIfBlocking`)
    ;[1 1 1] Set Placeholder ship materials.
    (for (_ _array_index) (`MeshComponent.GetMaterials` _placeholdershipmesh)
      (`PrimitiveComponent.SetMaterial` _placeholdershipmesh _array_index (select `bool` (`self.SomethingBlocking`) :`false` "/Game/Project/Asets/SpaceStation/Materials/Effects/MI_Placeholder_Valid.MI_Placeholder_Valid" :`true` "/Game/Project/Asets/SpaceStation/Materials/Effects/MI_Placeholder_Invalid.MI_Placeholder_Invalid" :!type "MaterialInterface Object Reference")))
    (`ActorComponent.K2_DestroyComponent` (`self.PlaceholderActor`))))