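; AI Vision component that gives non-AI owners a scan-and-tag view of actors implementing BI_UIData, reporting to a UI reference.
; While scanning, tick zooms the camera, drives an object-tracking post-process and sphere-traces to highlight a focus actor.
; A timer marks the focus with custom-depth stencils by collision type, a UI message and marker.
; A separate forward multi-sphere trace tags actors; looping timers flush highlights and tags.
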(event `InitializeAIVision`
  (params (UserInterfaceReference :type "/Game/Project/Asets/SpaceStation/Blueprints/UserInterface/Windows/WBP_SpacecraftMain Object Reference (by ref)") (CameraReference :type "CameraComponent Object Reference (by ref)") (IsAI :type Boolean))
  ;[1 1 1] Event Begin
  ;[1 1 1] Add AI Vision Widget to Viewport and Give Reference
  (set `self.IsAI` IsAI)
  (bind _output_get (set `self.UserInterfaceReference` UserInterfaceReference))
  (set `self.Camera` CameraReference)
  (set `/Game/Project/Asets/SpaceStation/Blueprints/UserInterface/Windows/WBP_SpacecraftMain.AIVisionRef` self _output_get)
  (if (not (`self.IsAI`))
    ;[1 1 1] Add Object Tracking Post Process Effect
    (bind _returnvalue (`KismetMaterialLibrary.CreateDynamicMaterialInstance` "/Game/Project/Asets/SpaceStation/Materials/MasterMaterials/Functions/MI_ObjectTracking.MI_ObjectTracking"))
    (set `self.PostProcessMaterialInstance` _returnvalue)
    (set `CameraComponent.PostProcessSettings` (make `PostProcessSettings` :`WeightedBlendables` (make `WeightedBlendables` (`|MakeArray` (make `WeightedBlendable` 1.0 (`self.PostProcessMaterialInstance`))))) (`self.Camera`))
    (`KismetSystemLibrary.K2_SetTimerDelegate` (delegate `ClearHighlightedActors`) 1.0 true)
    (`KismetSystemLibrary.K2_SetTimerDelegate` (delegate `ClearTags`) 10.0 true)
    ;[1 1 1] Set Tick enabled after short delay to avoid issues
    (`KismetSystemLibrary.Delay` 1.0)
    (`self.SetComponentTickEnabled` true)))

(event `self.ReceiveBeginPlay`)

(event `ClearHighlightedActors`
  ;[1 1 1] Flush HightlightedActors Array
  (`self.FlushHightlightedActors`))

(event `ClearTags`
  ;[1 1 1] Flush TaggedActors Array
  (`self.FlushTaggedActors`))

(event `self.ReceiveTick`
  (params (DeltaSeconds :type "Float (single-precision)"))
  (bind _returnvalue (`self.GetOwner`))
  (bind _camera (`self.Camera`))
  (bind _postprocessmaterialinstance (`self.PostProcessMaterialInstance`))
  (bind _userinterfacereference (`self.UserInterfaceReference`))
  (bind _camera_2 (`self.Camera`))
  (bind _camera_3 (`self.Camera`))
  (bind _returnvalue_2 (`SceneComponent.K2_GetComponentLocation` _camera_3))
  (bind _returnvalue_3 (`Actor.K2_GetActorLocation` _returnvalue))
  (bind _returnvalue_4 (`KismetMathLibrary.FInterpTo` (`CameraComponent.FieldOfView` _camera_2) (`self.MaxZoomFOV`) DeltaSeconds 1.0))
  (bind _returnvalue_5 (`KismetMathLibrary.FInterpTo` (`CameraComponent.FieldOfView` _camera_2) (`self.DefaultFOV`) DeltaSeconds 5.0))
  ;[1 1 1] Event Tick
  (if (not (`self.IsAI`))
    (`|ExecutionSequence`
      (:`then_0`
        (if (`self.Scanning`)
          (bind _output_get (set `self.ScanEffectCurrent` (`KismetMathLibrary.FInterpTo` (`self.ScanEffectCurrent`) 1500.0 DeltaSeconds 1.0)))
          (`MaterialInstanceDynamic.SetScalarParameterValue` _postprocessmaterialinstance "ScanDensityDistance" _output_get)
          (`CameraComponent.SetFieldOfView` _camera _returnvalue_4)
          (bind _output_get_2 (set `self.CurrentFOV` _returnvalue_4))
          (`/Game/Project/Asets/SpaceStation/Blueprints/UserInterface/Windows/WBP_SpacecraftMain.Scanning` _userinterfacereference _output_get_2 true)
          ;[1 1 1] Scanning Line
          (bind _outhit (`KismetSystemLibrary.SphereTraceSingle` (+ _returnvalue_2 (* (`SceneComponent.GetForwardVector` _camera_3) (`self.ScanningDistance`))) _returnvalue_2 500.0 "TraceTypeQuery1" false (`|MakeArray` (`self.GetOwner`))))
          (bind (_bblockinghit _binitialoverlap _time _distance _location _impactpoint _normal _impactnormal _physmat _hitactor) (`GameplayStatics.BreakHitResult` _outhit))
          ;[1 1 1] Actor Have Something That Contains UI Info
          (if _bblockinghit
            (if (and (`KismetSystemLibrary.DoesImplementInterface` _hitactor "/Game/Project/Asets/SpaceStation/Blueprints/UserInterface/Parent/BI_UIData.BI_UIData_C") (not (`KismetArrayLibrary.Array_Contains` (`self.MarkedActors`) _hitactor)))
              ;[1 1 1] First Hightlighting
              (bind _output_get_3 (set `self.FocalActor` _hitactor))
              (set `/Game/Project/Asets/SpaceStation/Blueprints/UserInterface/Windows/WBP_SpacecraftMain.FocusActor` _output_get_3 (`self.UserInterfaceReference`))
              (`self.ActorHightlighting`)
              ;[1 1 1] Then Scanning
              (`/Engine/EditorBlueprintResources/StandardMacros.IsValid` (`self.FocalActor`) :!label _label
                (:`Is Valid`
                  (`/Engine/EditorBlueprintResources/StandardMacros.DoOnce` false :!label _label_2
                    (:`Completed`
                      ;;[1 1 1] Mark Actor when ScanningTime is met
                      (`KismetSystemLibrary.K2_SetTimer` self "ActorMarking" (`self.ScanningTime`) true))))
                (:`Is Not Valid`
                  (goto _label_2 :!via `Reset`))))
            (else
              (set `self.FocalActor` null :!label _label_3)
              (goto _label)))
          (else
            (bind _output_get_4 (set `self.ScanEffectCurrent` (`KismetMathLibrary.FInterpTo` (`self.ScanEffectCurrent`) 0.0 DeltaSeconds 10.0)))
            (`MaterialInstanceDynamic.SetScalarParameterValue` _postprocessmaterialinstance "ScanDensityDistance" _output_get_4)
            (`CameraComponent.SetFieldOfView` _camera _returnvalue_5)
            (bind _output_get_5 (set `self.CurrentFOV` _returnvalue_5))
            (`/Game/Project/Asets/SpaceStation/Blueprints/UserInterface/Windows/WBP_SpacecraftMain.Scanning` _userinterfacereference _output_get_5 false)
            (goto _label_3))))
      (:`then_1`
        (if (`self.AllowTagging`)
          ;[1 1 1] Tagging Radius
          (bind _outhits (`KismetSystemLibrary.SphereTraceMulti` _returnvalue_3 (+ _returnvalue_3 (* (`Actor.GetActorForwardVector` _returnvalue) 8500.0)) (`self.TaggingRadius`) "TraceTypeQuery1" false (`|MakeArray` (`self.GetOwner`))))
          (for _array_element _outhits
            (bind (_bblockinghit_2 _binitialoverlap_2 _time_2 _distance_2 _location_2 _impactpoint_2 _normal_2 _impactnormal_2 _physmat_2 _hitactor_2 _hitcomponent) (`GameplayStatics.BreakHitResult` _array_element))
            (if _bblockinghit_2
              ;[1 1 1] Actor Have Something That Contains UI Info
              (if (and (`KismetSystemLibrary.DoesImplementInterface` _hitactor_2 "/Game/Project/Asets/SpaceStation/Blueprints/UserInterface/Parent/BI_UIData.BI_UIData_C") (not (`KismetArrayLibrary.Array_Contains` (`self.TaggedActors`) _hitactor_2)))
                ;[1 1 1] Add to TaggedActors Array
                (`KismetArrayLibrary.Array_Add` (`self.TaggedActors`) _hitactor_2)
                (`/Game/Project/Asets/SpaceStation/Blueprints/UserInterface/Windows/WBP_SpacecraftMain.Tagging` (`self.UserInterfaceReference`) (select `ECollisionChannel` (`PrimitiveComponent.GetCollisionObjectType` _hitcomponent) :`ECC_WorldStatic` 2 :`ECC_WorldDynamic` 2 :`ECC_Pawn` 4 :`ECC_Visibility` 2 :`ECC_Camera` 2 :`ECC_PhysicsBody` 3 :`ECC_Vehicle` 4 :`ECC_Destructible` 2))))))))))

(fn `ActorHightlighting`
  (bind _focalactor (`self.FocalActor`))
  (for _array_element (`Actor.K2_GetComponentsByClass` _focalactor "/Script/Engine.PrimitiveComponent")
    ;[1 1 1] Set FocalActor custom depth values
    (`PrimitiveComponent.SetRenderCustomDepth` _array_element true)
    (`PrimitiveComponent.SetCustomDepthStencilValue` _array_element 1))
  ;[1 1 1] Add to HightlightedActors Array
  (`KismetArrayLibrary.Array_Add` (`self.HighlightedActors`) _focalactor))

(fn `ActorMarking`
  (bind _focalactor (`self.FocalActor`))
  (`/Engine/EditorBlueprintResources/StandardMacros.IsValid` _focalactor
    (:`Is Valid`
      (if (not (`KismetArrayLibrary.Array_Contains` (`self.MarkedActors`) _focalactor))
        (message `/Game/Project/Asets/SpaceStation/Blueprints/UserInterface/Parent/BI_UIData.OpenUI` _focalactor)
        (for _array_element (`Actor.K2_GetComponentsByClass` _focalactor "/Script/Engine.PrimitiveComponent")
          ;[1 1 1] Set FocalActor custom depth values
          (`PrimitiveComponent.SetRenderCustomDepth` _array_element true)
          (bind _returnvalue (select `ECollisionChannel` (`PrimitiveComponent.GetCollisionObjectType` _array_element) :`ECC_WorldStatic` 2 :`ECC_WorldDynamic` 2 :`ECC_Pawn` 4 :`ECC_Visibility` 2 :`ECC_Camera` 2 :`ECC_PhysicsBody` 3 :`ECC_Vehicle` 4 :`ECC_Destructible` 2))
          (`PrimitiveComponent.SetCustomDepthStencilValue` _array_element _returnvalue)
          ;[1 1 1] Add UI Marking
          (`/Engine/EditorBlueprintResources/StandardMacros.DoOnce` false :!label _label
            (:`Completed`
              (`/Game/Project/Asets/SpaceStation/Blueprints/UserInterface/Windows/WBP_SpacecraftMain.Marking` (`self.UserInterfaceReference`) _returnvalue))))
        ;[1 1 1] Remove from HightlightedActors Array and add to MarkedActors Arra
        (`KismetArrayLibrary.Array_RemoveItem` (`self.HighlightedActors`) _focalactor)
        (`KismetArrayLibrary.Array_Add` (`self.MarkedActors`) _focalactor)
        (goto _label :!via `Reset`)))))

(fn `FlushHightlightedActors`
  ;[1 1 1] Flush Hightlighted Actors
  (`/Engine/EditorBlueprintResources/StandardMacros.IsValid` (`self.Camera`)
    (:`Is Valid`
      (for _array_element (`self.HighlightedActors`)
        (for _array_element_2 (`Actor.K2_GetComponentsByClass` _array_element "/Script/Engine.PrimitiveComponent")
          (`PrimitiveComponent.SetRenderCustomDepth` _array_element_2 false)))
      (`KismetArrayLibrary.Array_Clear` (`self.HighlightedActors`)))))

(fn `FlushMarkedActors`
  ;[1 1 1] Flush Marked Actors
  (for _array_element (`self.MarkedActors`)
    (`/Engine/EditorBlueprintResources/StandardMacros.IsValid` _array_element
      (:`Is Valid`
        (message `/Game/Project/Asets/SpaceStation/Blueprints/UserInterface/Parent/BI_UIData.HideUI` _array_element)
        (for _array_element_2 (`Actor.K2_GetComponentsByClass` _array_element "/Script/Engine.PrimitiveComponent")
          (`PrimitiveComponent.SetRenderCustomDepth` _array_element_2 false)))))
  (`KismetArrayLibrary.Array_Clear` (`self.MarkedActors`))
  (`/Game/Project/Asets/SpaceStation/Blueprints/UserInterface/Windows/WBP_SpacecraftMain.ClearCompass` (`self.UserInterfaceReference`))
  (`self.FlushTaggedActors`))

(fn `FlushTaggedActors`
  ;[1 1 1] Flush Marked Actors
  (`KismetArrayLibrary.Array_Clear` (`self.TaggedActors`))
  (`/Game/Project/Asets/SpaceStation/Blueprints/UserInterface/Windows/WBP_SpacecraftMain.ClearTags` (`self.UserInterfaceReference`)))