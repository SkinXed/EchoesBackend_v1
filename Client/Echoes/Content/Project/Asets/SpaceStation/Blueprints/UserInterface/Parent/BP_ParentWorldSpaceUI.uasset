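; Parent actor for world-space UI widgets in the space station project, with an optional beam line linking the widget to a target object.
; Construction applies widget placement, pivot and scale, plus line color and thickness.
; While the widget is visible, Tick zeroes root rotation, optionally billboards the widget toward the camera and moves the particle beam's endpoints to the line source and target.
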(event `self.ReceiveBeginPlay`
  (bind _widgetlineparticle (`self.WidgetLineParticle`))
  ;[1 1 1] Toggle Line Visibility
  (if (`self.UseLine`)
    (`SceneComponent.SetVisibility` _widgetlineparticle true false)
    ;[1 1 1] Line Updating
    (`ParticleSystemComponent.SetBeamSourcePoint` (`self.WidgetLineParticle`) 0 (0.0 0.0 0.0) 0)
    (`ParticleSystemComponent.SetBeamTargetPoint` (`self.WidgetLineParticle`) 0 (0.0 0.0 0.0) 0)
    (else
      (`SceneComponent.SetVisibility` _widgetlineparticle false false))))

(event `self.ReceiveTick`
  (params (DeltaSeconds :type "Float (single-precision)"))
  (bind _widget (`self.Widget`))
  (if (`self.WidgetVisible`)
    (`SceneComponent.K2_SetWorldRotation` :`self` (`self.DefaultSceneRoot`))
    (if (`self.UseBillboard`)
      ;[1 1 1] WidgetBillboard
      (`SceneComponent.K2_SetWorldRotation` _widget (`KismetMathLibrary.FindLookAtRotation` (`SceneComponent.K2_GetComponentLocation` _widget) (`PlayerCameraManager.GetCameraLocation` (`GameplayStatics.GetPlayerCameraManager` 0))) false false))
    (if (`self.UseLine`)
      ;[1 1 1] Line Updating
      (`ParticleSystemComponent.SetBeamSourcePoint` (`self.WidgetLineParticle`) 0 (`SceneComponent.K2_GetComponentLocation` (`self.LineSourceUI`)) 0)
      (`ParticleSystemComponent.SetBeamTargetPoint` (`self.WidgetLineParticle`) 0 (`SceneComponent.K2_GetComponentLocation` (`self.LineTargetObject`)) 0))))

(fn `InitUIAppearance`
  (bind _linethickness (`self.LineThickness`))
  (bind _widget (`self.Widget`))
  (bind _uicolor (`self.UIColor`))
  (bind (_uix_ylocation_x _uix_ylocation_y) (`KismetMathLibrary.BreakVector2D` (`self.UIX&YLocation`)))
  (bind _widgetlineparticle (`self.WidgetLineParticle`))
  (`SceneComponent.K2_SetRelativeLocation` (`self.Widget`) (`KismetMathLibrary.MakeVector` _uix_ylocation_x _uix_ylocation_y (`self.UIDeviation`)) false false)
  (`WidgetComponent.SetPivot` _widget (`KismetMathLibrary.MakeVector2D` (`self.UIPivotX`) (`self.UIPivotY`)))
  (`SceneComponent.SetWorldScale3D` _widget (`self.UIScale`))
  ;[1 1 1] Set Line Color
  (`FXSystemComponent.SetVectorParameter` _widgetlineparticle "Color" (`KismetMathLibrary.MakeVector` (break `LinearColor` (break `/Game/Project/Asets/SpaceStation/Blueprints/UserInterface/Parent/S_UIColors` _uicolor)) (`.G` (break `LinearColor` (break `/Game/Project/Asets/SpaceStation/Blueprints/UserInterface/Parent/S_UIColors` _uicolor))) (`.B` (break `LinearColor` (break `/Game/Project/Asets/SpaceStation/Blueprints/UserInterface/Parent/S_UIColors` _uicolor)))))
  ;[1 1 1] Set Line Thickness
  (`FXSystemComponent.SetVectorParameter` _widgetlineparticle "LineSize" (`KismetMathLibrary.MakeVector` _linethickness _linethickness _linethickness)))

(fn `UserConstructionScript`
  (`self.InitUIAppearance`))