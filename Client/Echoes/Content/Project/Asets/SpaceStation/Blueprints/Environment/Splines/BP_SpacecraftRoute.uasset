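; Spline route actor that fills a path with ambient spacecraft traffic, using either static meshes or child actors.
; CreateTraffic runs in the construction script, using a seeded stream for model choice, spline position, offset and speed factor.
; On Tick, RunTraffic advances normalized spline positions, wrapping at the ends and supporting reversed direction.
; Only actor mode applies per-craft speed factors; it also configures BP_ParentSpacecraft children as non-player traffic with random appearance.
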(event `self.ReceiveBeginPlay`
  (`parent.ReceiveBeginPlay`))

(event `self.ReceiveTick`
  (params (DeltaSeconds :type "Float (single-precision)"))
  (bind _returnvalue (* DeltaSeconds (`self.TrafficSpeed`)))
  ;[1 1 1] Move Traffic
  (if (`self.TrafficEnabled`)
    (`self.RunTraffic` (select `bool` (`self.TrafficReverse`) :`false` _returnvalue :`true` (* _returnvalue -1.0)))))

(fn `CreateTraffic`
  (locals (LocalSpacecraftSplineLocation :type "Float (double-precision)") (LocalSpacecraftOffset :type "Vector Structure") (LocalSpacecraftSpeedFactor :type "Float (double-precision)"))
  (bind _spline (`self.Spline`))
  (bind _trafficoffset (`self.TrafficOffset`))
  (bind _returnvalue (`KismetMathLibrary.RandomFloatInRangeFromStream` (`self.RandomSeedStruct`) (* -1 _trafficoffset) _trafficoffset))
  (bind _returnvalue_2 (`KismetMathLibrary.Lerp` 0.0 (`SplineComponent.GetSplineLength` _spline) (`local.LocalSpacecraftSplineLocation`)))
  (bind _returnvalue_3 (`SplineComponent.GetRotationAtDistanceAlongSpline` _spline _returnvalue_2 "Local"))
  (bind _returnvalue_4 (select `bool` (`self.TrafficReverse`) :`false` _returnvalue_3 :`true` (`KismetMathLibrary.MakeRotFromXY` (* (`KismetMathLibrary.GetForwardVector` _returnvalue_3) -1) (* (`KismetMathLibrary.GetRightVector` _returnvalue_3) -1))))
  ;[1 1 1] Array Clearing
  (`KismetArrayLibrary.Array_Clear` (`self.AddedSpacecraftSplineLocations`))
  (`KismetArrayLibrary.Array_Clear` (`self.AddedSpacecraftsMeshes`))
  (`KismetArrayLibrary.Array_Clear` (`self.AddedSpacecraftOffset`))
  (`KismetArrayLibrary.Array_Clear` (`self.AddedSpacecraftSpeedFactors`))
  (if (`self.UseSpacecraftActorsInstead`)
    ;[1 1 1] Add Spacecraft Actors And Set Variables
    (for _ (range (`self.NumberOfSpacecrafts`))
      (bind _returnvalue_5 (`AddComponent|NODE_AddChildActorComponent-0`))
      (`KismetArrayLibrary.Array_Add` (`self.AddedSpacecraftActors`) _returnvalue_5)
      (`ChildActorComponent.SetChildActorClass` _returnvalue_5 (`|GetArrayItem` (`self.SpacecraftActors`) (`KismetMathLibrary.RandomIntegerInRangeFromStream` (`self.RandomSeedStruct`) 0 (`KismetArrayLibrary.Array_Length` (`self.SpacecraftActors`)))))
      (bind _asbp_parent_spacecraft (cast `/Game/Project/Asets/SpaceStation/Blueprints/SpaceCrafts/Parent/BP_ParentSpacecraft` (`ChildActorComponent.ChildActor` _returnvalue_5))
        (:`then`
          (set `/Game/Project/Asets/SpaceStation/Blueprints/SpaceCrafts/Parent/BP_ParentSpacecraft.TrafficMode` true _asbp_parent_spacecraft)
          (set `/Game/Project/Asets/SpaceStation/Blueprints/SpaceCrafts/Parent/BP_ParentSpacecraft.NonPlayerMode` true _asbp_parent_spacecraft)
          (set `/Game/Project/Asets/SpaceStation/Blueprints/SpaceCrafts/Parent/BP_ParentSpacecraft.UseRandomAppearance` true _asbp_parent_spacecraft)
          (set `/Game/Project/Asets/SpaceStation/Blueprints/SpaceCrafts/Parent/BP_ParentSpacecraft.ForwardSpeedCurrent` (select `bool` (`self.TrafficEnabled`) :`true` 3000.0) _asbp_parent_spacecraft)
          (`/Game/Project/Asets/SpaceStation/Blueprints/SpaceCrafts/Parent/BP_ParentSpacecraft.SetVisuals` _asbp_parent_spacecraft))
        (:`CastFailed`
          _))
      ;[1 1 1] Random Location from Spline
      (bind _output_get (set `local.LocalSpacecraftSplineLocation` (`KismetMathLibrary.RandomFloatInRangeFromStream` (`self.RandomSeedStruct`) 0.0 1.0) :!label _label))
      (`KismetArrayLibrary.Array_Add` (`self.AddedSpacecraftSplineLocations`) _output_get)
      ;[1 1 1] Random Offset from Spline
      (bind _output_get_2 (set `local.LocalSpacecraftOffset` (`KismetMathLibrary.MakeVector` _returnvalue _returnvalue _returnvalue)))
      (`KismetArrayLibrary.Array_Add` (`self.AddedSpacecraftOffset`) _output_get_2)
      ;[1 1 1] Random Speed Factors
      (`KismetArrayLibrary.Array_Add` (`self.AddedSpacecraftSpeedFactors`) (`KismetMathLibrary.RandomFloatInRangeFromStream` (`self.RandomSeedStruct`) (`self.TrafficSpeedSlowFactor`) (`self.TrafficSpeedFastFactor`)))
      (bind _returnvalue_6 (select `bool` (`self.UseSpacecraftActorsInstead`) :`false` (stale _returnvalue_7) :`true` _returnvalue_5 :!type "SceneComponent Object Reference"))
      (`/Engine/EditorBlueprintResources/StandardMacros.IsValid` _returnvalue_6
        (:`Is Valid`
          (`SceneComponent.K2_SetRelativeLocationAndRotation` _returnvalue_6 (+ (`SplineComponent.GetLocationAtDistanceAlongSpline` _spline _returnvalue_2 "Local") (`KismetMathLibrary.GreaterGreater_VectorRotator` (`local.LocalSpacecraftOffset`) _returnvalue_4)) _returnvalue_4 false false))))
    (else
      ;[1 1 1] Add Spacecraft Meshes
      (for _ (range (`self.NumberOfSpacecrafts`))
        (bind _returnvalue_7 (`AddComponent|NODE_AddStaticMeshComponent-0`))
        (`KismetArrayLibrary.Array_Add` (`self.AddedSpacecraftsMeshes`) _returnvalue_7)
        (`StaticMeshComponent.SetStaticMesh` _returnvalue_7 (`|GetArrayItem` (`self.SpacecraftMeshes`) (`KismetMathLibrary.RandomIntegerInRangeFromStream` (`self.RandomSeedStruct`) 0 (`KismetArrayLibrary.Array_Length` (`self.SpacecraftMeshes`)))))
        (goto _label)))))

(fn `RunTraffic`
  (params (TrafficPosition :type "Float (double-precision)"))
  (locals (LocalSplineLocation :type "Float (double-precision)"))
  (bind _spline (`self.Spline`))
  (bind _addedspacecraftsplinelocations (`self.AddedSpacecraftSplineLocations`))
  (bind _addedspacecraftsplinelocations_2 (`self.AddedSpacecraftSplineLocations`))
  (bind _spline_2 (`self.Spline`))
  (bind _trafficreverse (`self.TrafficReverse`))
  (bind _trafficreverse_2 (`self.TrafficReverse`))
  (if (`self.UseSpacecraftActorsInstead`)
    ;[1 1 1] Move Spaceship Actors
    (for (_array_element _array_index) (`self.AddedSpacecraftActors`)
      (bind _returnvalue (+ (`|GetArrayItem` _addedspacecraftsplinelocations _array_index) (* TrafficPosition (`|GetArrayItem` (`self.AddedSpacecraftSpeedFactors`) _array_index))))
      (bind _output_get (set `local.LocalSplineLocation` _returnvalue))
      (`KismetArrayLibrary.Array_Remove` _addedspacecraftsplinelocations _array_index)
      (`KismetArrayLibrary.Array_Insert` _addedspacecraftsplinelocations _output_get _array_index)
      (if (select `bool` _trafficreverse_2 :`false` (>= _returnvalue 1.0) :`true` (<= _returnvalue 0.0))
        (`KismetArrayLibrary.Array_Remove` _addedspacecraftsplinelocations _array_index)
        (`KismetArrayLibrary.Array_Insert` _addedspacecraftsplinelocations (select `bool` _trafficreverse_2 :`true` 1.0) _array_index))
      (bind _returnvalue_2 (`KismetMathLibrary.Lerp` 0.0 (`SplineComponent.GetSplineLength` _spline) (`|GetArrayItem` _addedspacecraftsplinelocations _array_index)))
      (bind _returnvalue_3 (`SplineComponent.GetRotationAtDistanceAlongSpline` _spline _returnvalue_2 "Local"))
      (bind _returnvalue_4 (select `bool` (`self.TrafficReverse`) :`false` _returnvalue_3 :`true` (`KismetMathLibrary.MakeRotFromXY` (* (`KismetMathLibrary.GetForwardVector` _returnvalue_3) -1) (* (`KismetMathLibrary.GetRightVector` _returnvalue_3) -1))))
      (`SceneComponent.K2_SetRelativeLocation` _array_element (+ (`SplineComponent.GetLocationAtDistanceAlongSpline` _spline _returnvalue_2 "Local") (`KismetMathLibrary.GreaterGreater_VectorRotator` (`|GetArrayItem` (`self.AddedSpacecraftOffset`) _array_index) _returnvalue_4)) false false)
      (`SceneComponent.K2_SetRelativeRotation` _array_element _returnvalue_4 false false))
    (else
      ;[1 1 1] Move Spaceship Meshes
      (for (_array_element_2 _array_index_2) (`self.AddedSpacecraftsMeshes`)
        (bind _returnvalue_5 (+ (`|GetArrayItem` _addedspacecraftsplinelocations_2 _array_index_2) TrafficPosition))
        (bind _output_get_2 (set `local.LocalSplineLocation` _returnvalue_5))
        (`KismetArrayLibrary.Array_Remove` _addedspacecraftsplinelocations_2 _array_index_2)
        (`KismetArrayLibrary.Array_Insert` _addedspacecraftsplinelocations_2 _output_get_2 _array_index_2)
        (if (select `bool` _trafficreverse :`false` (>= _returnvalue_5 1.0) :`true` (<= _returnvalue_5 0.0))
          (`KismetArrayLibrary.Array_Remove` _addedspacecraftsplinelocations_2 _array_index_2)
          (`KismetArrayLibrary.Array_Insert` _addedspacecraftsplinelocations_2 (select `bool` _trafficreverse :`true` 1.0) _array_index_2))
        (bind _returnvalue_6 (`KismetMathLibrary.Lerp` 0.0 (`SplineComponent.GetSplineLength` _spline_2) (`|GetArrayItem` _addedspacecraftsplinelocations_2 _array_index_2)))
        (bind _returnvalue_7 (`SplineComponent.GetRotationAtDistanceAlongSpline` _spline_2 _returnvalue_6 "Local"))
        (bind _returnvalue_8 (select `bool` (`self.TrafficReverse`) :`false` _returnvalue_7 :`true` (`KismetMathLibrary.MakeRotFromXY` (* (`KismetMathLibrary.GetForwardVector` _returnvalue_7) -1) (* (`KismetMathLibrary.GetRightVector` _returnvalue_7) -1))))
        (`SceneComponent.K2_SetRelativeLocation` _array_element_2 (+ (`SplineComponent.GetLocationAtDistanceAlongSpline` _spline_2 _returnvalue_6 "Local") (`KismetMathLibrary.GreaterGreater_VectorRotator` (`|GetArrayItem` (`self.AddedSpacecraftOffset`) _array_index_2) _returnvalue_8)) false false)
        (`SceneComponent.K2_SetRelativeRotation` _array_element_2 _returnvalue_8 false false)))))

(fn `UserConstructionScript`
  (`parent.UserConstructionScript`)
  (`self.CreateTraffic`))