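; Spline-route actor that scatters asteroid meshes along a spline and moves them along it as an animated environment stream.
; The construction script spawns the meshes from a seeded random stream, each with its own mesh, scale, rotation, spline position, offset and speed factor stored in parallel arrays.
; Tick advances each normalized position, forward or reversed, wraps it at the spline ends, and re-places the mesh using the spline's orientation.
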(event `self.ReceiveBeginPlay`
  (`parent.ReceiveBeginPlay`))

(event `self.ReceiveTick`
  (params (DeltaSeconds :type "Float (single-precision)"))
  (bind _returnvalue (* DeltaSeconds (`self.MovementSpeed`)))
  (if (`self.MovingAsteroidsEnabled`)
    (`self.MoveAsteroids` (select `bool` (`self.MovementReverse`) :`false` _returnvalue :`true` (* _returnvalue -1.0)))))

(fn `CreateMovingAsteroids`
  (locals (LocalAsteroidOffset :type "Vector Structure") (LocalAsteroidSplineLocation :type "Float (double-precision)") (LocalAsteroidRotation :type "Rotator Structure"))
  (bind _spline (`self.Spline`))
  (bind _locationoffset (`self.LocationOffset`))
  (bind _returnvalue (`KismetMathLibrary.RandomFloatInRangeFromStream` (`self.RandomSeedStruct`) (* -1 _locationoffset) _locationoffset))
  (bind _returnvalue_2 (`KismetMathLibrary.Lerp` 0.0 (`SplineComponent.GetSplineLength` _spline) (`local.LocalAsteroidSplineLocation`)))
  (bind _returnvalue_3 (`SplineComponent.GetRotationAtDistanceAlongSpline` _spline _returnvalue_2 "Local"))
  (bind _returnvalue_4 (`KismetMathLibrary.ComposeRotators` (select `bool` (`self.MovementReverse`) :`false` _returnvalue_3 :`true` (`KismetMathLibrary.MakeRotFromXY` (* (`KismetMathLibrary.GetForwardVector` _returnvalue_3) -1) (* (`KismetMathLibrary.GetRightVector` _returnvalue_3) -1))) (`local.LocalAsteroidRotation`)))
  ;[1 1 1] Array Clearing
  (`KismetArrayLibrary.Array_Clear` (`self.AddedAsteroidsSplineLocations`))
  (`KismetArrayLibrary.Array_Clear` (`self.AddedAsteroidsMeshes`))
  (`KismetArrayLibrary.Array_Clear` (`self.AddedAsteroidsOffset`))
  (`KismetArrayLibrary.Array_Clear` (`self.AddedAsteroidsSpeedFactors`))
  (`KismetArrayLibrary.Array_Clear` (`self.AddedAsteroidsRotations`))
  ;[1 1 1] Add Asteroid Meshes
  (for _ (range (`self.NumberOfAsteroids`))
    (bind _output_get (set `local.LocalAsteroidRotation` (`KismetMathLibrary.RandomRotatorFromStream` (`self.RandomSeedStruct`) true)))
    (`KismetArrayLibrary.Array_Add` (`self.AddedAsteroidsRotations`) _output_get)
    (bind _returnvalue_5 (`AddComponent|NODE_AddStaticMeshComponent-0` :`RelativeTransform` (`KismetMathLibrary.MakeTransform` (0.0 0.0 0.0) (`local.LocalAsteroidRotation`) (* (`KismetMathLibrary.MakeVector` 1.0 1.0 1.0) (`KismetMathLibrary.RandomFloatInRangeFromStream` (`self.RandomSeedStruct`) (`self.AsteroidMinScale`) (`self.AsteroidMaxScale`))))))
    (`KismetArrayLibrary.Array_Add` (`self.AddedAsteroidsMeshes`) _returnvalue_5)
    (`StaticMeshComponent.SetStaticMesh` _returnvalue_5 (`|GetArrayItem` (`self.AsteroidMeshes`) (`KismetMathLibrary.RandomIntegerInRangeFromStream` (`self.RandomSeedStruct`) 0 (`KismetArrayLibrary.Array_Length` (`self.AsteroidMeshes`)))))
    ;[1 1 1] Random Location from Spline
    (bind _output_get_2 (set `local.LocalAsteroidSplineLocation` (`KismetMathLibrary.RandomFloatInRangeFromStream` (`self.RandomSeedStruct`) 0.0 1.0)))
    (`KismetArrayLibrary.Array_Add` (`self.AddedAsteroidsSplineLocations`) _output_get_2)
    ;[1 1 1] Random Offset from Spline
    (bind _output_get_3 (set `local.LocalAsteroidOffset` (`KismetMathLibrary.MakeVector` _returnvalue _returnvalue _returnvalue)))
    (`KismetArrayLibrary.Array_Add` (`self.AddedAsteroidsOffset`) _output_get_3)
    ;[1 1 1] Random Speed Factors
    (`KismetArrayLibrary.Array_Add` (`self.AddedAsteroidsSpeedFactors`) (`KismetMathLibrary.RandomFloatInRangeFromStream` (`self.RandomSeedStruct`) (`self.AsteroidsSpeedSlowFactor`) (`self.AsteroidsSpeedFastFactor`)))
    (`/Engine/EditorBlueprintResources/StandardMacros.IsValid` _returnvalue_5
      (:`Is Valid`
        (`SceneComponent.K2_SetRelativeLocationAndRotation` _returnvalue_5 (+ (`SplineComponent.GetLocationAtDistanceAlongSpline` _spline _returnvalue_2 "Local") (`KismetMathLibrary.GreaterGreater_VectorRotator` (`local.LocalAsteroidOffset`) _returnvalue_4)) _returnvalue_4 false false)))))

(fn `MoveAsteroids`
  (params (AsteroidsPosition :type "Float (double-precision)"))
  (locals (LocalSplineLocation :type "Float (double-precision)"))
  (bind _movementreverse (`self.MovementReverse`))
  (bind _addedasteroidssplinelocations (`self.AddedAsteroidsSplineLocations`))
  (bind _spline (`self.Spline`))
  ;[1 1 1] Move Asteroids Meshes
  (for (_array_element _array_index) (`self.AddedAsteroidsMeshes`)
    (bind _returnvalue (+ (`|GetArrayItem` _addedasteroidssplinelocations _array_index) (* AsteroidsPosition (`|GetArrayItem` (`self.AddedAsteroidsSpeedFactors`) _array_index))))
    (bind _output_get (set `local.LocalSplineLocation` _returnvalue))
    (`KismetArrayLibrary.Array_Remove` _addedasteroidssplinelocations _array_index)
    (`KismetArrayLibrary.Array_Insert` _addedasteroidssplinelocations _output_get _array_index)
    (if (select `bool` _movementreverse :`false` (>= _returnvalue 1.0) :`true` (<= _returnvalue 0.0))
      (`KismetArrayLibrary.Array_Remove` _addedasteroidssplinelocations _array_index)
      (`KismetArrayLibrary.Array_Insert` _addedasteroidssplinelocations (select `bool` _movementreverse :`true` 1.0) _array_index))
    (bind _returnvalue_2 (`KismetMathLibrary.Lerp` 0.0 (`SplineComponent.GetSplineLength` _spline) (`|GetArrayItem` _addedasteroidssplinelocations _array_index)))
    (bind _returnvalue_3 (`SplineComponent.GetRotationAtDistanceAlongSpline` _spline _returnvalue_2 "Local"))
    (bind _returnvalue_4 (`KismetMathLibrary.ComposeRotators` (select `bool` (`self.MovementReverse`) :`false` _returnvalue_3 :`true` (`KismetMathLibrary.MakeRotFromXY` (* (`KismetMathLibrary.GetForwardVector` _returnvalue_3) -1) (* (`KismetMathLibrary.GetRightVector` _returnvalue_3) -1))) (`|GetArrayItem` (`self.AddedAsteroidsRotations`) _array_index)))
    (`SceneComponent.K2_SetRelativeLocation` _array_element (+ (`SplineComponent.GetLocationAtDistanceAlongSpline` _spline _returnvalue_2 "Local") (`KismetMathLibrary.GreaterGreater_VectorRotator` (`|GetArrayItem` (`self.AddedAsteroidsOffset`) _array_index) _returnvalue_4)) false false)
    (`SceneComponent.K2_SetRelativeRotation` _array_element _returnvalue_4 false false)))

(fn `UserConstructionScript`
  (`parent.UserConstructionScript`)
  (if (`self.MovingAsteroidsEnabled`)
    (`self.CreateMovingAsteroids`)))