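; Parent Blueprint for floating space station items that randomizes their look and item data at construction, with no runtime logic of its own.
; After the parent construction script, InitFloatingMesh picks a mesh, scale and optional rotation, then caches the world transform.
; An optional flag also randomizes weight, quantity and class in ItemData.
; All rolls draw from RandomStream, so variation is seed-driven.
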(event `self.ReceiveBeginPlay`)

(fn `InitFloatingMesh`
  (bind _meshes (`self.Meshes`))
  (bind _returnvalue (* (1.0 1.0 1.0) (`KismetMathLibrary.RandomFloatInRangeFromStream` (`self.RandomStream`) (`self.MinScale`) (`self.MaxScale`))))
  ;[1 1 1] Choose Random Mesh From Array
  (`StaticMeshComponent.SetStaticMesh` (`self.ItemMesh`) (`|GetArrayItem` _meshes (`KismetMathLibrary.RandomIntegerInRangeFromStream` (`self.RandomStream`) 0 (- (`KismetArrayLibrary.Array_Length` _meshes) 1))))
  ;[1 1 1] Random Scale
  (`SceneComponent.SetWorldScale3D` (`self.ItemMesh`) _returnvalue)
  (set `self.Scale` _returnvalue)
  ;[1 1 1] Random Rotation
  (`SceneComponent.K2_SetWorldRotation` (`self.ItemMesh`) (`KismetMathLibrary.ComposeRotators` (select `bool` (`self.RandomRotation`) :`true` (`KismetMathLibrary.RandomRotatorFromStream` (`self.RandomStream`) true)) (`self.K2_GetActorRotation`)) false false)
  (set `self.MeshWorldTransform` (`SceneComponent.K2_GetComponentToWorld` (`self.ItemMesh`))))

(fn `UserConstructionScript`
  (bind (_itemdata_itemname _itemdata_itemweight _itemdata_itemquantity _itemdata_itemdescription _itemdata_itemclass) (break `/Game/Project/Asets/SpaceStation/Blueprints/Items/Parent/S_ItemData` (`self.ItemData`)))
  (bind (_itemdata_itemname_2 _itemdata_itemweight_2 _itemdata_itemquantity_2 _itemdata_itemdescription_2 _itemdata_itemclass_2 _itemdata_itemtype _itemdata_interactable _itemdata_itemicon) (break `/Game/Project/Asets/SpaceStation/Blueprints/Items/Parent/S_ItemData` (`self.ItemData`)))
  (`parent.UserConstructionScript`)
  (`self.InitFloatingMesh`)
  ;[1 1 1] Random Item Data
  (set `self.ItemData` (make `/Game/Project/Asets/SpaceStation/Blueprints/Items/Parent/S_ItemData` _itemdata_itemname_2 (select `bool` (`self.RandomItemValues`) :`false` _itemdata_itemweight :`true` (`KismetMathLibrary.RandomIntegerInRangeFromStream` (`self.RandomStream`) (`self.ItemWeightRandomMin`) (`self.ItemWeightRandomMax`))) (select `bool` (`self.RandomItemValues`) :`false` _itemdata_itemquantity :`true` (`KismetMathLibrary.RandomIntegerInRangeFromStream` (`self.RandomStream`) (`self.ItemQuantityRandomMin`) (`self.ItemQuantityRandomMax`))) _itemdata_itemdescription_2 (select `bool` (`self.RandomItemValues`) :`false` _itemdata_itemclass_2 :`true` (cast `/Game/Project/Asets/SpaceStation/Blueprints/Items/Parent/E_ItemClass` (`KismetMathLibrary.Conv_IntToByte` (`KismetMathLibrary.RandomIntegerInRangeFromStream` (`self.RandomStream`) 0 (`KismetArrayLibrary.Array_Length` (`|MakeArray` _itemdata_itemclass)))))) _itemdata_itemtype _itemdata_interactable _itemdata_itemicon)))