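; Parent space station light Blueprint that drives a light mesh and its child light components, with optional steady or random flashing.
; The construction script creates a dynamic material for the mesh and applies the color and on/off state to it and the lights.
; When flashing, a looping timer toggles light visibility, gated by a weighted coin flip in random mode, and updates the emissive color to match.
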(event `self.ReceiveBeginPlay`
  ;[1 1 1] Is Light Flashing
  (if (`self.FlashingLight`)
    (`KismetSystemLibrary.K2_SetTimerDelegate` (delegate `BlinkLight`) (select `bool` (`self.RandomFlashing`) :`false` (`self.FlashDelay`) :`true` 0.5) true)))

(event `BlinkLight`
  (if (`self.RandomFlashing`)
    (if (`KismetMathLibrary.RandomBoolWithWeight` 0.65)
      ;[1 1 1] Set Light Visibility
      (for _array_element (`SceneComponent.GetChildrenComponents` (`self.Lights`) false) :!label _label
        (bind _aslight_component (cast `LightComponent` _array_element))
        (bind _bvisible (`SceneComponent.bVisible` _aslight_component))
        (`SceneComponent.SetVisibility` _aslight_component (not _bvisible) false)
        (set `self.LightOn` _bvisible))
      ;[1 1 1] Set Light Material Color
      (`MaterialInstanceDynamic.SetVectorParameterValue` (`self.LightMatInst`) "EmissiveColor" (select `bool` (`self.LightOn`) :`true` (`self.LightColor`))))
    (else
      (goto _label))))

(fn `UserConstructionScript`
  (bind _lightmesh (`self.LightMesh`))
  ;[1 1 1] Change Light Material Color
  (bind _returnvalue (`PrimitiveComponent.CreateDynamicMaterialInstance` _lightmesh 1 (`PrimitiveComponent.GetMaterial` _lightmesh 1) "None"))
  (set `self.LightMatInst` _returnvalue)
  (`MaterialInstanceDynamic.SetVectorParameterValue` (`self.LightMatInst`) "EmissiveColor" (select `bool` (`self.LightOn`) :`true` (`self.LightColor`)))
  ;[1 1 1] Set Light Colors
  (for _array_element (`SceneComponent.GetChildrenComponents` (`self.Lights`) false)
    (bind _aslight_component (cast `LightComponent` _array_element))
    (`LightComponent.SetLightColor` _aslight_component (`self.LightColor`) true)
    (`SceneComponent.SetVisibility` _aslight_component (select `bool` (`self.LightOn`) :`true` true) false)))