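; BP_Transporter is a space station wormhole device that sends spacecraft to a named destination.
; Overlapping the entering point while the device is unbroken stores the spacecraft and marks it usable until exit.
; UseDevice then delegates to the game controller's EnterWormhole, passing destination, spacecraft, itself and exit point; the controller is looked up after a delay at BeginPlay.
; Tick counter-rotates three sets of rings and lights while powered and unbroken.
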(event `self.ReceiveBeginPlay`
  (`parent.ReceiveBeginPlay`)
  ;[1 1 1] Get GameManager Reference
  (`KismetSystemLibrary.Delay` 1.0)
  (bind _outactors (`GameplayStatics.GetAllActorsOfClass` "/Game/Project/Asets/SpaceStation/Blueprints/GameControl/BP_GameController.BP_GameController_C"))
  (set `self.SpaceGameManagerRef` (`|GetArrayItem` _outactors)))

(event `Rotate OnServer`
  ;[1 1 1] Ring1Rotation
  (`SceneComponent.K2_AddLocalRotation` (`self.Rotators1`) (`KismetMathLibrary.MakeRotator` 0.0 (* (`GameplayStatics.GetWorldDeltaSeconds`) 10.0)) false false)
  (`SceneComponent.K2_AddLocalRotation` (`self.Ring1Lights`) (`KismetMathLibrary.MakeRotator` 0.0 (* (`GameplayStatics.GetWorldDeltaSeconds`) 10.0)) false false)
  ;[1 1 1] Ring2Rotation
  (`SceneComponent.K2_AddLocalRotation` (`self.Ring2Lights`) (`KismetMathLibrary.MakeRotator` 0.0 (* (* (`GameplayStatics.GetWorldDeltaSeconds`) 10.0) -1.0)) false false)
  (`SceneComponent.K2_AddLocalRotation` (`self.Rotators2`) (`KismetMathLibrary.MakeRotator` 0.0 (* (* (`GameplayStatics.GetWorldDeltaSeconds`) 10.0) -1.0)) false false)
  ;[1 1 1] Ring3Rotation
  (`SceneComponent.K2_AddLocalRotation` (`self.Rotators3`) (`KismetMathLibrary.MakeRotator` 0.0 (* (`GameplayStatics.GetWorldDeltaSeconds`) 5.0)) false false)
  (`SceneComponent.K2_AddLocalRotation` (`self.Ring3Lights`) (`KismetMathLibrary.MakeRotator` 0.0 (* (`GameplayStatics.GetWorldDeltaSeconds`) 5.0)) false false))

(event `self.ReceiveTick`
  (params (DeltaSeconds :type "Float (single-precision)"))
  (`parent.ReceiveTick` DeltaSeconds)
  (if (`self.IsBroken`)
    _
    (elif (`self.IsPoweredOn`)
      (`self.Rotate OnServer`))))

(event `self.EnteringPoint.OnComponentBeginOverlap`
  (params (OverlappedComponent :type "PrimitiveComponent Object Reference") (OtherActor :type "Actor Object Reference") (OtherComp :type "PrimitiveComponent Object Reference") (OtherBodyIndex :type Integer) (bFromSweep :type Boolean) (SweepResult :type "HitResult Structure (by ref)"))
  ;[1 1 1] Player Entering Wormhole
  (if (not (`self.IsBroken`))
    (bind _asbp_parent_spacecraft (cast `/Game/Project/Asets/SpaceStation/Blueprints/SpaceCrafts/Parent/BP_ParentSpacecraft` OtherActor))
    (set `self.SpaceshipReference` _asbp_parent_spacecraft)
    (set `self.IsUsableState` true)))

(event `self.EnteringPoint.OnComponentEndOverlap`
  (params (OverlappedComponent :type "PrimitiveComponent Object Reference") (OtherActor :type "Actor Object Reference") (OtherComp :type "PrimitiveComponent Object Reference") (OtherBodyIndex :type Integer))
  ;[1 1 1] Player Leaving Wormhole
  (cast `/Game/Project/Asets/SpaceStation/Blueprints/SpaceCrafts/Parent/BP_ParentSpacecraft` OtherActor)
  (set `self.IsUsableState` false))

(event `/Game/Project/Asets/SpaceStation/Blueprints/Structure/Device/Parent/BI_Device.UseDevice`
  ;[1 1 1] Use Wormhole When Player is inside, Device Powered On and not Broken
  (`parent.UseDevice`)
  (if (`self.IsUsableState`)
    (`/Engine/EditorBlueprintResources/StandardMacros.IsValid` (`self.SpaceGameManagerRef`)
      (:`Is Valid`
        (`/Game/Project/Asets/SpaceStation/Blueprints/GameControl/BP_GameController.EnterWormhole` (`self.SpaceGameManagerRef`) (`self.DestinationLocationName`) (`self.SpaceshipReference`) self (`self.ExitingPoint`))))))

(fn `UserConstructionScript`
  (`parent.UserConstructionScript`))