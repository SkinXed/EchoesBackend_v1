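; BP_HotStar is a visual star actor built from a star body, horizontal and vertical corona plates, and sun flare components.
; Its Construction Script creates a dynamic material instance for each component and stores it in a variable.
; Blueprint variables then drive the body's Kelvin colors, plasma flow, atmosphere, storms, tessellation and vertex animation, plus shared corona and flare colors.
; The event graph has no active logic, so the Blueprint does no runtime work.
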(fn `UserConstructionScript`
  (bind _returnvalue (`PrimitiveComponent.CreateDynamicMaterialInstance` (`self.StarHot`) 0 null "None"))
  (bind _output_get (set `self.Star_DM_B` _returnvalue))
  (bind _returnvalue_2 (`PrimitiveComponent.CreateDynamicMaterialInstance` (`self.CPlateHorizontal_A`) 0 null "None"))
  (bind _output_get_2 (set `self.Star_Plate_A` _returnvalue_2))
  (bind _returnvalue_3 (`PrimitiveComponent.CreateDynamicMaterialInstance` (`self.CPlateHorizontal_B`) 0 null "None"))
  (bind _output_get_3 (set `self.Star_Plate_B` _returnvalue_3))
  (bind _returnvalue_4 (`PrimitiveComponent.CreateDynamicMaterialInstance` (`self.CPlateHorizontal_C`) 0 null "None"))
  (bind _output_get_4 (set `self.Star_Plate_C` _returnvalue_4))
  (bind _returnvalue_5 (`PrimitiveComponent.CreateDynamicMaterialInstance` (`self.CPlateHorizontal_D`) 0 null "None"))
  (bind _output_get_5 (set `self.Star_Plate_D` _returnvalue_5))
  (bind _returnvalue_6 (`PrimitiveComponent.CreateDynamicMaterialInstance` (`self.CPlateVerticle_A`) 0 null "None"))
  (bind _output_get_6 (set `self.Star_VPlate_A` _returnvalue_6))
  (bind _returnvalue_7 (`PrimitiveComponent.CreateDynamicMaterialInstance` (`self.CPlateVerticle_B`) 0 null "None"))
  (bind _output_get_7 (set `self.Star_VPlate_B` _returnvalue_7))
  (bind _returnvalue_8 (`PrimitiveComponent.CreateDynamicMaterialInstance` (`self.CPlateVerticle_C`) 0 null "None"))
  (bind _output_get_8 (set `self.Star_VPlate_C` _returnvalue_8))
  (bind _returnvalue_9 (`PrimitiveComponent.CreateDynamicMaterialInstance` (`self.CPlateVerticle_D`) 0 null "None"))
  (bind _output_get_9 (set `self.Star_VPlate_D` _returnvalue_9))
  (bind _returnvalue_10 (`PrimitiveComponent.CreateDynamicMaterialInstance` (`self.SunFlare_A`) 0 null "None"))
  (bind _output_get_10 (set `self.Star_Flare_A` _returnvalue_10))
  (bind _returnvalue_11 (`PrimitiveComponent.CreateDynamicMaterialInstance` (`self.SunFlare_B`) 0 null "None"))
  (bind _output_get_11 (set `self.Star_Flare_B` _returnvalue_11))
  (bind _returnvalue_12 (`PrimitiveComponent.CreateDynamicMaterialInstance` (`self.SunFlare_C`) 0 null "None"))
  (bind _output_get_12 (set `self.Star_Flare_C` _returnvalue_12))
  (bind _returnvalue_13 (`PrimitiveComponent.CreateDynamicMaterialInstance` (`self.SunFlare_D`) 0 null "None"))
  (bind _output_get_13 (set `self.Star_Flare_D` _returnvalue_13))
  (bind _returnvalue_14 (`PrimitiveComponent.CreateDynamicMaterialInstance` (`self.SunFlare_E`) 0 null "None"))
  (bind _output_get_14 (set `self.Star_Flare_E` _returnvalue_14))
  (bind _returnvalue_15 (`PrimitiveComponent.CreateDynamicMaterialInstance` (`self.SunFlare_F`) 0 null "None"))
  (bind _output_get_15 (set `self.Star_Flare_F` _returnvalue_15))
  (bind _returnvalue_16 (`PrimitiveComponent.CreateDynamicMaterialInstance` (`self.SunFlare_G`) 0 null "None"))
  (bind _output_get_16 (set `self.Star_Flare_G` _returnvalue_16))
  (bind _returnvalue_17 (`PrimitiveComponent.CreateDynamicMaterialInstance` (`self.SunFlare_H`) 0 null "None"))
  (bind _output_get_17 (set `self.Star_Flare_H` _returnvalue_17))
  (bind _returnvalue_18 (`PrimitiveComponent.CreateDynamicMaterialInstance` (`self.SunFlare_I`) 0 null "None"))
  (bind _output_get_18 (set `self.Star_Flare_I` _returnvalue_18))
  (bind _returnvalue_19 (`PrimitiveComponent.CreateDynamicMaterialInstance` (`self.SunFlare_J`) 0 null "None"))
  (bind _output_get_19 (set `self.Star_Flare_J` _returnvalue_19))
  (`MaterialInstanceDynamic.SetVectorParameterValue` _output_get_10 "FlareColor" (`self.Flare_KelvinOffset`))
  (`MaterialInstanceDynamic.SetVectorParameterValue` _output_get_11 "FlareColor" (`self.Flare_KelvinOffset`))
  (`MaterialInstanceDynamic.SetVectorParameterValue` _output_get_12 "FlareColor" (`self.Flare_KelvinOffset`))
  (`MaterialInstanceDynamic.SetVectorParameterValue` _output_get_13 "FlareColor" (`self.Flare_KelvinOffset`))
  (`MaterialInstanceDynamic.SetVectorParameterValue` _output_get_14 "FlareColor" (`self.Flare_KelvinOffset`))
  (`MaterialInstanceDynamic.SetVectorParameterValue` _output_get_15 "FlareColor" (`self.Flare_KelvinOffset`))
  (`MaterialInstanceDynamic.SetVectorParameterValue` _output_get_16 "FlareColor" (`self.Flare_KelvinOffset`))
  (`MaterialInstanceDynamic.SetVectorParameterValue` _output_get_17 "FlareColor" (`self.Flare_KelvinOffset`))
  (`MaterialInstanceDynamic.SetVectorParameterValue` _output_get_18 "FlareColor" (`self.Flare_KelvinOffset`))
  (`MaterialInstanceDynamic.SetVectorParameterValue` _output_get_19 "FlareColor" (`self.Flare_KelvinOffset`))
  (`MaterialInstanceDynamic.SetVectorParameterValue` _output_get "KH_AtmoHot" (`self.Atmosphere_Kelvin`))
  (`MaterialInstanceDynamic.SetVectorParameterValue` _output_get "KH_SurfaceCool" (`self.SurfaceKelvin_Cool`))
  (`MaterialInstanceDynamic.SetVectorParameterValue` _output_get "KH_SurfaceWarm" (`self.SurfaceKelvin_Warm`))
  (`MaterialInstanceDynamic.SetVectorParameterValue` _output_get "KH_SurfaceHot" (`self.SurfaceKelvin_Hot`))
  (`MaterialInstanceDynamic.SetVectorParameterValue` _output_get "SurfaceActivity_Bleed" (`self.Surface_Bleed`))
  (`MaterialInstanceDynamic.SetVectorParameterValue` _output_get "SurfaceActivity_Center" (`self.Surface_Spot`))
  (`MaterialInstanceDynamic.SetScalarParameterValue` _output_get "3DCoord_FlowTile" (`self.Fluid_Resolution`))
  (`MaterialInstanceDynamic.SetScalarParameterValue` _output_get "3DFlowNormal_Power" (`self.Fluid_Density`))
  (`MaterialInstanceDynamic.SetScalarParameterValue` _output_get "3DPlasmaFlow_Speed" (`self.Fluid_Speed`))
  (`MaterialInstanceDynamic.SetScalarParameterValue` _output_get "3DSurface_Offset" (`self.Surface_Offset`))
  (`MaterialInstanceDynamic.SetScalarParameterValue` _output_get "DistAtmo_Falloff" (`self.Atmosphere_Curve`))
  (`MaterialInstanceDynamic.SetScalarParameterValue` _output_get "DistAtmo_Power" (`self.Atmosphere_Density`))
  (`MaterialInstanceDynamic.SetScalarParameterValue` _output_get "FluidActivity_Influence" (`self.StormSurface_Blend`))
  (`MaterialInstanceDynamic.SetScalarParameterValue` _output_get "SolarActivity_InnerFalloff" (`self.StormIn_Curve`))
  (`MaterialInstanceDynamic.SetScalarParameterValue` _output_get "SolarActivity_OutsideFalloff" (`self.StormOut_Curve`))
  (`MaterialInstanceDynamic.SetScalarParameterValue` _output_get "Tessellation_Resolution" (`self.Tessellation_Resolution`))
  (`MaterialInstanceDynamic.SetScalarParameterValue` _output_get "Vertex_Speed" (`self.VertexSpeed_Animation`))
  (`MaterialInstanceDynamic.SetScalarParameterValue` _output_get "VertexOffset_Falloff" (`self.Vertex_Curve`))
  (`MaterialInstanceDynamic.SetScalarParameterValue` _output_get "VertexOffset_Power" (`self.Vertex_Power`))
  (`MaterialInstanceDynamic.SetScalarParameterValue` _output_get "VertexOffset_Tile" (`self.Vertex_Resolution`))
  (`MaterialInstanceDynamic.SetVectorParameterValue` _output_get_2 "CoronaKelvin_Hot" (`self.Corona_Kelvin`))
  (`MaterialInstanceDynamic.SetVectorParameterValue` _output_get_3 "CoronaKelvin_Hot" (`self.Corona_Kelvin`))
  (`MaterialInstanceDynamic.SetVectorParameterValue` _output_get_4 "CoronaKelvin_Hot" (`self.Corona_Kelvin`))
  (`MaterialInstanceDynamic.SetVectorParameterValue` _output_get_5 "CoronaKelvin_Hot" (`self.Corona_Kelvin`))
  (`MaterialInstanceDynamic.SetVectorParameterValue` _output_get_6 "CoronaKelvin_Hot" (`self.Corona_Kelvin`))
  (`MaterialInstanceDynamic.SetVectorParameterValue` _output_get_7 "CoronaKelvin_Hot" (`self.Corona_Kelvin`))
  (`MaterialInstanceDynamic.SetVectorParameterValue` _output_get_9 "CoronaKelvin_Hot" (`self.Corona_Kelvin`))
  (`MaterialInstanceDynamic.SetVectorParameterValue` _output_get_8 "CoronaKelvin_Hot" (`self.Corona_Kelvin`)))