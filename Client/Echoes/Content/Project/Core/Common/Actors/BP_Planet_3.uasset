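; Configurable gas-giant-style planet actor with banded clouds, storms, lightning, polar auroras, two atmosphere shells and rings, built entirely in the Construction Script.
; It creates dynamic material instances for each component and pushes the actor's appearance variables into their parameters.
; A valid LightSource actor's forward vector drives lighting, negated for the second atmosphere shell.
; Atmosphere shells are scaled from planet size plus AtmosphereHeight only when that light is valid.
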(fn `UserConstructionScript`
  (bind _light_source (`self.Light_Source`))
  (bind _atmosphere_1_material (`self.Atmosphere_1_Material`))
  (bind _planet_material (`self.Planet_Material`))
  (bind _atmosphere_color (`self.Atmosphere Color`))
  (bind _atmosphere_brightness (`self.Atmosphere Brightness`))
  (bind _rings_material (`self.Rings_Material`))
  (bind _ringcomponent (`self.RingComponent`))
  (bind _planet_material_2 (`self.Planet_Material`))
  (bind _atmosphere_falloff (`self.Atmosphere Falloff`))
  (bind _planet_material_3 (`self.Planet_Material`))
  (bind _atmosphere_2_material (`self.Atmosphere_2_Material`))
  (bind _planet_material_4 (`self.Planet_Material`))
  (bind _returnvalue (* (`self.Atmosphere Falloff`) 120.0))
  (bind _returnvalue_2 (`KismetMathLibrary.Conv_RotatorToVector` (`self.K2_GetActorRotation` _light_source)))
  (bind _returnvalue_3 (+ (`SceneComponent.K2_GetComponentScale` (`self.Planet`)) (`self.Atmosphere Height`)))
  (bind _returnvalue_4 (`KismetMathLibrary.Conv_VectorToLinearColor` _returnvalue_2))
  (bind _returnvalue_5 (`PrimitiveComponent.CreateDynamicMaterialInstance` (`self.Planet`) 0 (`self.Material_Instance_Planet`) "None"))
  (set `self.Planet_Material` _returnvalue_5)
  (bind _returnvalue_6 (`PrimitiveComponent.CreateDynamicMaterialInstance` (`self.Atmosphere_1`) 0 (`self.Material_Instance_Atmosphere`) "None"))
  (set `self.Atmosphere_1_Material` _returnvalue_6)
  (bind _returnvalue_7 (`PrimitiveComponent.CreateDynamicMaterialInstance` (`self.Atmosphere_2`) 0 (`self.Material_Instance_Atmosphere`) "None"))
  (set `self.Atmosphere_2_Material` _returnvalue_7)
  (bind _returnvalue_8 (`PrimitiveComponent.CreateDynamicMaterialInstance` _ringcomponent 0 (`PrimitiveComponent.GetMaterial` _ringcomponent 0) "None"))
  (set `self.Rings_Material` _returnvalue_8)
  (`|ExecutionSequence`
    (:`then_0`
      (`MaterialInstanceDynamic.SetVectorParameterValue` (`self.Planet_Material`) "Atmosphere_Color" _atmosphere_color)
      (`MaterialInstanceDynamic.SetVectorParameterValue` _atmosphere_1_material "Atmosphere_Color" _atmosphere_color)
      (`MaterialInstanceDynamic.SetScalarParameterValue` _atmosphere_1_material "Atmosphere_Brightness" _atmosphere_brightness)
      (`MaterialInstanceDynamic.SetScalarParameterValue` (`self.Planet_Material`) "Atmosphere_Brightness" _atmosphere_brightness)
      (`MaterialInstanceDynamic.SetScalarParameterValue` _atmosphere_1_material "InnerBredth" _atmosphere_falloff)
      (`MaterialInstanceDynamic.SetScalarParameterValue` _atmosphere_1_material "InnerBredth" _returnvalue)
      (`MaterialInstanceDynamic.SetScalarParameterValue` (`self.Planet_Material`) "Atmosphere_Falloff" (* (`self.Atmosphere Inner Falloff`) 2.0)))
    (:`then_1`
      (`MaterialInstanceDynamic.SetVectorParameterValue` _atmosphere_2_material "Atmosphere_Color" _atmosphere_color)
      (`MaterialInstanceDynamic.SetScalarParameterValue` _atmosphere_2_material "Atmosphere_Brightness" _atmosphere_brightness)
      (`MaterialInstanceDynamic.SetScalarParameterValue` _atmosphere_2_material "InnerBredth" _atmosphere_falloff)
      (`MaterialInstanceDynamic.SetScalarParameterValue` _atmosphere_2_material "InnerBredth" _returnvalue))
    (:`then_2`
      (`MaterialInstanceDynamic.SetScalarParameterValue` _planet_material_3 "Strip_Frequency" (`self.Strip Frequency`))
      (`MaterialInstanceDynamic.SetScalarParameterValue` _planet_material_3 "Zone_Frequency" (`self.Zone Frequency`))
      (`MaterialInstanceDynamic.SetScalarParameterValue` _planet_material_3 "Clouds_Speed_X" (`self.Clouds Speed X`))
      (`MaterialInstanceDynamic.SetScalarParameterValue` _planet_material_3 "Clouds_Speed_Y" (`self.Clouds Speed Y`))
      (`MaterialInstanceDynamic.SetScalarParameterValue` _planet_material_3 "Zone_1_Style" (`self.Zone 1 Style`))
      (`MaterialInstanceDynamic.SetScalarParameterValue` _planet_material_3 "Zone_2_Style" (`self.Zone 2 Style`))
      (`MaterialInstanceDynamic.SetScalarParameterValue` _planet_material_3 "Clouds_Coverage" (`self.Clouds Coverage`))
      (`MaterialInstanceDynamic.SetScalarParameterValue` _planet_material_3 "Color_Frequency" (`self.Color Frequency`))
      (`MaterialInstanceDynamic.SetScalarParameterValue` _planet_material_3 "Clouds_Rougness" (`self.Clouds Rougness`))
      (`MaterialInstanceDynamic.SetScalarParameterValue` _planet_material_3 "Extinction_intensity" (`self.Extinction Intensity`))
      (`MaterialInstanceDynamic.SetVectorParameterValue` _planet_material_3 "Fast_Color_1" (`self.Fast Deep Color`))
      (`MaterialInstanceDynamic.SetVectorParameterValue` _planet_material_3 "Fast_Color_2" (`self.Fast Clouds Color `))
      (`MaterialInstanceDynamic.SetVectorParameterValue` _planet_material_3 "Slow_Color_1" (`self.Slow Deep Color`))
      (`MaterialInstanceDynamic.SetVectorParameterValue` _planet_material_3 "Slow_Color_2" (`self.Slow Clouds Color`))
      (`MaterialInstanceDynamic.SetVectorParameterValue` _planet_material_3 "Extinction_Color" (`self.Extinction Color`))
      (`MaterialInstanceDynamic.SetTextureParameterValue` _planet_material_3 "Cloud_Mask" (`self.Cloud Mask`)))
    (:`then_3`
      (`MaterialInstanceDynamic.SetScalarParameterValue` _planet_material_4 "Turbolence_Intensity" (`self.Turbolence Intensity`))
      (`MaterialInstanceDynamic.SetScalarParameterValue` _planet_material_4 "Storm_Zone_Frequency" (`self.Storm Zone Frequency`))
      (`MaterialInstanceDynamic.SetScalarParameterValue` _planet_material_4 "Storm_Frequency" (`self.Storm Size`))
      (`MaterialInstanceDynamic.SetScalarParameterValue` _planet_material_4 "Storm_Intensity_1" (`self.Storm Intensity 1`))
      (`MaterialInstanceDynamic.SetScalarParameterValue` _planet_material_4 "Storm_Intensity_2" (`self.Storm Intensity 2`))
      (`MaterialInstanceDynamic.SetScalarParameterValue` _planet_material_4 "Lightning_Brightness" (`self.Lightning Brigtness`))
      (`MaterialInstanceDynamic.SetVectorParameterValue` _planet_material_4 "Lightning_Color" (`self.Lightning Color`))
      (`MaterialInstanceDynamic.SetTextureParameterValue` _planet_material_4 "Storm_Texture" (`self.Storm Mask`)))
    (:`then_4`
      (`MaterialInstanceDynamic.SetScalarParameterValue` _planet_material "Polar_Storm" (`self.Polar Storm`))
      (`MaterialInstanceDynamic.SetScalarParameterValue` _planet_material "Poles_Clouds_Speed" (`self.Polar Clouds Speed`))
      (`MaterialInstanceDynamic.SetScalarParameterValue` _planet_material "Aurora_Brightness" (`self.Aurora_Brightness`))
      (`MaterialInstanceDynamic.SetVectorParameterValue` _planet_material "Poles_Color_1" (`self.Poles Clouds Color`))
      (`MaterialInstanceDynamic.SetVectorParameterValue` _planet_material "Poles_Color_2" (`self.Poles Deep Color`))
      (`MaterialInstanceDynamic.SetVectorParameterValue` _planet_material "Aurora_Color_1" (`self.Aurora Color 1`))
      (`MaterialInstanceDynamic.SetVectorParameterValue` _planet_material "Aurora_Color_2" (`self.Aurora Color 2`)))
    (:`then_5`
      (`MaterialInstanceDynamic.SetScalarParameterValue` _rings_material "Inner_FallOff" (`self.Rings Inner Falloff`))
      (`MaterialInstanceDynamic.SetScalarParameterValue` _rings_material "Outer_FallOff" (`self.Rings Outer Falloff`))
      (`MaterialInstanceDynamic.SetScalarParameterValue` _rings_material "Opacity" (`self.Rings Opacity`))
      (`MaterialInstanceDynamic.SetScalarParameterValue` _rings_material "Ring_Frequency" (`self.Rings Frequency`))
      (`MaterialInstanceDynamic.SetScalarParameterValue` _rings_material "Ring_Color_Frequency" (`self.Rings Color Frequency`))
      (`MaterialInstanceDynamic.SetScalarParameterValue` _rings_material "Opacity_Mask_Power" (`self.Rings Opacity Mask Power`))
      (`MaterialInstanceDynamic.SetScalarParameterValue` _rings_material "Color_Mask_power" (`self.Rings Color Mask Power`))
      (`MaterialInstanceDynamic.SetScalarParameterValue` _rings_material "Ring_Density" (`self.Rings Density`))
      (`MaterialInstanceDynamic.SetVectorParameterValue` _rings_material "Color_1" (`self.Ring Color 1`))
      (`MaterialInstanceDynamic.SetVectorParameterValue` _rings_material "Color_2" (`self.Ring Color 2`)))
    (:`then_6`
      (`MaterialInstanceDynamic.SetScalarParameterValue` _planet_material_2 "High_Belt_Coverage" (`self.High Bands Coverage`))
      (`MaterialInstanceDynamic.SetScalarParameterValue` _planet_material_2 "High_Belt_Frequency" (`self.High Bands Frequency`))
      (`MaterialInstanceDynamic.SetScalarParameterValue` _planet_material_2 "High_Belt_Speed" (`self.High Bands Speed`))
      (`MaterialInstanceDynamic.SetVectorParameterValue` _planet_material_2 "High_Belt_Color_1" (`self.High Bands Color 1`))
      (`MaterialInstanceDynamic.SetVectorParameterValue` _planet_material_2 "High_Belt_Color_2" (`self.High Bands Color 2`))
      (`MaterialInstanceDynamic.SetTextureParameterValue` _planet_material_2 "High_Belt_Texture" (`self.High Bands Texture`))
      (`MaterialInstanceDynamic.SetTextureParameterValue` _planet_material_2 "High_Belt_Mask" (`self.High Bands Mask`)))
    (:`then_7`
      (`/Engine/EditorBlueprintResources/StandardMacros.IsValid` _light_source
        (:`Is Valid`
          (`MaterialInstanceDynamic.SetVectorParameterValue` (`self.Atmosphere_1_Material`) "LightDirection" _returnvalue_4)
          (`MaterialInstanceDynamic.SetVectorParameterValue` (`self.Atmosphere_2_Material`) "LightDirection" (`KismetMathLibrary.Conv_VectorToLinearColor` (`KismetMathLibrary.MakeVector` (* (.x _returnvalue_2) -1.0) (* (.y _returnvalue_2) -1.0) (* (.z _returnvalue_2) -1.0))))
          (`MaterialInstanceDynamic.SetVectorParameterValue` (`self.Planet_Material`) "Light_Direction" _returnvalue_4)
          (`SceneComponent.SetWorldScale3D` (`self.Atmosphere_1`) _returnvalue_3)
          (`SceneComponent.SetWorldScale3D` (`self.Atmosphere_2`) _returnvalue_3)
          (set `self.Refresh Material` false))))))